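; BP_TootBot is a player-controlled bot that moves and looks via Enhanced Input, adding IMC_TootBot on possession.
; Shortly after BeginPlay it passes a fixed landscape size to its Niagara component, then its XY location, refreshed on move input as the paint location.
; An outline post-process setup using M_SceneOutlineEffect is present but disconnected, leaving AddPostProcessEfft empty.
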(event `self.ReceivePossessed`
  (params (NewController :type "Controller Object Reference"))
  (bind _asplayer_controller (cast `PlayerController` NewController))
  (`EnhancedInputSubsystemInterface.AddMappingContext` (pcsubsystem `EnhancedInputLocalPlayerSubsystem` _asplayer_controller) "/Game/Inputs/IMC_TootBot.IMC_TootBot" 0 (struct)))

(event `self.ReceiveBeginPlay`
  (`self.AddPostProcessEfft`)
  (`self.NsKeepLandscapeSz`))

(event `AddPostProcessEfft`)

(event `self.ReceiveTick`
  (params (DeltaSeconds :type "Float (single-precision)")))

(event `NsKeepLandscapeSz`
  (`KismetSystemLibrary.Delay` 0.2)
  (`NiagaraComponent.SetVariableVec2` (`self.Niagara`) "LandscapeSz" (50400.0 31400.0))
  (`self.UpdPaintLocation`))

(event `UpdPaintLocation`
  (bind (_returnvalue_x _returnvalue_y) (`KismetMathLibrary.BreakVector` (`self.K2_GetActorLocation`)))
  (`NiagaraComponent.SetVariableVec2` (`self.Niagara`) "CurrBotLoc" (`KismetMathLibrary.MakeVector2D` _returnvalue_x _returnvalue_y)))

(event `EnhancedInput|/Game/Inputs/IA_TootBotMove`
  (params (ActionValue :type "Vector2D Structure") (ElapsedSeconds :type "Float (double-precision)") (TriggeredSeconds :type "Float (double-precision)") (InputAction :type "InputAction Object Reference" :default "/Game/Inputs/IA_TootBotMove.IA_TootBotMove"))
  (bind (_returnvalue_roll _returnvalue_pitch _returnvalue_yaw) (`KismetMathLibrary.BreakRotator` (`self.GetControlRotation`)))
  (bind (_returnvalue_roll_2 _returnvalue_pitch_2 _returnvalue_yaw_2) (`KismetMathLibrary.BreakRotator` (`self.GetControlRotation`)))
  (:`Triggered`
    (`self.AddMovementInput` (`KismetMathLibrary.GetRightVector` (`KismetMathLibrary.MakeRotator` _returnvalue_roll_2 0.0 _returnvalue_yaw_2)) ActionValue_Y)
    (`self.AddMovementInput` (`KismetMathLibrary.GetForwardVector` (`KismetMathLibrary.MakeRotator` 0.0 0.0 _returnvalue_yaw)) ActionValue_X)
    (`self.UpdPaintLocation`)))

(event `EnhancedInput|/Game/Inputs/IA_TootBotLook`
  (params (ActionValue :type "Vector2D Structure") (ElapsedSeconds :type "Float (double-precision)") (TriggeredSeconds :type "Float (double-precision)") (InputAction :type "InputAction Object Reference" :default "/Game/Inputs/IA_TootBotLook.IA_TootBotLook"))
  (:`Triggered`
    (`self.AddControllerYawInput` ActionValue_X)
    (`self.AddControllerPitchInput` ActionValue_Y)))

(fn `UserConstructionScript`)